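; Inventory actor component that handles item pickup and dropping, along with the inventory, interaction prompt and item amount widgets.
; Items are stored as a class array with one entry per stack unit, and the open inventory widget is recreated after changes.
; Pickup draws from overlapping items, destroying the actor via a server event and optionally multicasting its sound.
; Drops server-spawn the stack ahead of the owner with random scatter.
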(event Custom|SERVER_SpawnItem
  (params (Class :type Actor%20Class%20Reference) (SpawnTransform :type Transform) (CurrentStack :type Integer))
  (bind _returnvalue (Game|SpawnActorfromClass Class SpawnTransform "AdjustIfPossibleButAlwaysSpawn" 0 0))
  (Development|PrintString "Item dropped.")
  ;[1 1 1] Interface This
  (bind _asbp_master_item (Utilities|Casting|CastToBP_MasterItem _returnvalue))
  (Variables|/Game/Components/Inventory/BP_MasterItem.BP_MasterItem_C|SetCurrentStack _asbp_master_item CurrentStack))

(event Custom|CLIENT_SpawnItem
  (params (Class :type Actor%20Class%20Reference) (SpawnTransform :type Transform))
  (CallFunction|SERVERSpawnItem Class SpawnTransform))

(event Custom|MC_PlaySound
  (params (Sound :type Sound%20Base%20Object%20Reference) (Location :type Vector))
  (Audio|PlaySoundatLocation Sound Location "0, 0, 0" 1.0 1.0 0.0 0 0 0 0))

(event Custom|SERVER_PlaySound
  (params (Sound :type Sound%20Base%20Object%20Reference) (Location :type Vector))
  (CallFunction|MCPlaySound Sound Location))

(event Custom|SERVER_DestroyActor
  (params (Actor%20To%20Destroy :type Actor%20Object%20Reference))
  (Actor|DestroyActor Actor%20To%20Destroy))

(event EventBeginPlay
  (Utilities|FlowControl|Delay 0.2)
  (Variables|Default|SetOwningActor (Components|GetOwner)))

(event EventSpawnItem
  (params (ItemToSpawn :type BP%20Master%20Item%20Class%20Reference) (Transform :type Transform)))

(event EventTick
  (params (DeltaSeconds :type Float%20%28single-precision%29)))

(fn ShowInventory
  (bind _returnvalue (Game|GetPlayerController 0))
  (if (and (not (Variables|Default|GetInventoryOpen?)) (Pawn|IsLocalPlayerController _returnvalue))
    (bind _returnvalue_2 (UserInterface|CreateWidget "/Game/Components/Inventory/WB_Inventory.WB_Inventory_C" _returnvalue))
    (Variables|Default|SetWB%20Inventory _returnvalue_2)
    (UserInterface|Viewport|AddtoViewport _returnvalue_2 0)
    (Default|UpdateInventory _returnvalue_2 (Variables|Default|GetInventory))
    (Variables|Default|SetInventoryOpen? true)
    (if (not (Variables|Default|GetUseController?))
      (Input|SetInputModeGameandUI (Game|GetPlayerController 0) (Variables|Default|GetWB%20Inventory) "LockInFullscreen" true)
      (Variables|/Script/Engine.PlayerController|SetbShowMouseCursor (Game|GetPlayerController 0) true))))

(fn HideInventory
  (CallFunction|ClearWidget (Variables|Default|GetWB%20Inventory))
  (Variables|Default|SetWB%20Inventory 0)
  (Variables|Default|SetInventoryOpen? false)
  (if (not (Variables|Default|GetUseController?))
    (Input|SetInputModeGameOnly (Game|GetPlayerController 0))
    (Variables|/Script/Engine.PlayerController|SetbShowMouseCursor (Game|GetPlayerController 0) false)))

(fn AddItemtoInventory
  (params (Item%20To%20Add :type BP%20Master%20Item%20Object%20Reference%20%28by%20ref%29))
  (bind _staticmesh (Variables|/Game/Components/Inventory/BP_MasterItem.BP_MasterItem_C|GetStaticMesh Item%20To%20Add))
  (bind _returnvalue (Transformation|GetWorldLocation _staticmesh))
  (Utilities|FlowControl|Sequence
    (:then_0
      (Utilities|Array|Add (Variables|Default|GetInventory) (Utilities|GetClass Item%20To%20Add))
      (if (Variables|Default|GetReplicatePickupSound)
        (Networking|SwitchHasAuthority
          (:Authority
            (CallFunction|MCPlaySound (Variables|Default|GetPickupSound) _returnvalue))
          (:Remote
            (CallFunction|SERVERPlaySound (Variables|Default|GetPickupSound) _returnvalue)))
        (else
          (Audio|PlaySoundatLocation (Variables|Default|GetPickupSound) _returnvalue "0, 0, 0" 1.0 1.0 0.0 0 0 0 0))))
    (:then_1
      (if (Variables|Default|GetInventoryOpen?)
        (CallFunction|HideInventory)
        (CallFunction|ShowInventory)))))

(fn DropItemfromInventory
  (params (ItemToSpawn :type BP%20Master%20Item%20Class%20Reference) (CurrentStack :type Integer))
  (bind _returnvalue (Components|GetOwner))
  (bind _inventory (Variables|Default|GetInventory))
  (Utilities|FlowControl|Sequence
    (:then_0
      (if (not (Utilities|Array|ContainsItem (Variables|Default|GetInventory) ItemToSpawn))
        (return)))
    (:then_1
      (LocalVariables|SetDropPosition (Math|Conversions|ToTransform(Vector) (+ (+ (Transformation|GetActorLocation _returnvalue) (* (Math|Vector|GetForwardVector (Transformation|GetActorRotation _returnvalue)) (Variables|Default|GetItemDropDistance))) (Math|Vector|MakeVector (Math|Random|RandomFloatinRange 5e+01 3e+02) (Math|Random|RandomFloatinRange 5e+01 3e+02) (Math|Float|SelectFloat (Math|Random|RandomFloatinRange 1e+01 4e+01) 0.0 (.SimulatePhysics? (Utilities|GetClassDefaults ItemToSpawn)))))))
      (CallFunction|SERVERSpawnItem ItemToSpawn (LocalVariables|GetDropPosition) CurrentStack)
      (for _index (range 1 CurrentStack)
        (Utilities|Array|RemoveIndex _inventory (Utilities|Array|FindItem _inventory ItemToSpawn)))
      (bind _wb_inventory (Variables|Default|GetWB%20Inventory)
        (:then
          (CallFunction|HideInventory)
          (CallFunction|ShowInventory))
        (:else)))))

(fn ShowInteraction
  (if (Pawn|IsLocalPlayerController (Game|GetPlayerController 0))
    (CallFunction|ClearWidget (Variables|Default|GetWB%20InteractionRef))
    (bind _returnvalue (UserInterface|CreateWidget "/Game/Components/Inventory/WB_Interaction.WB_Interaction_C"))
    (Variables|Default|SetWB%20InteractionRef _returnvalue)
    (UserInterface|Viewport|AddtoViewport (Variables|Default|GetWB%20InteractionRef) 0)
    (return)))

(fn HideInteraction
  (CallFunction|ClearWidget (Variables|Default|GetWB%20InteractionRef))
  (Variables|Default|SetWB%20InteractionRef 0)
  (return))

(fn TryPickupItem
  (bind _overlappingitems (Variables|Default|GetOverlappingItems))
  (Utilities|FlowControl|Sequence
    (:then_0
      (if (> (Utilities|Array|Length (Variables|Default|GetOverlappingItems)) 0)
        (for _index (range 1 (Variables|/Game/Components/Inventory/BP_MasterItem.BP_MasterItem_C|GetCurrentStack (Variables|Default|GetItemToPickup)))
          (CallFunction|AddItemtoInventory (Variables|Default|GetItemToPickup)))
        (Utilities|Array|RemoveItem (Variables|Default|GetOverlappingItems) (Variables|Default|GetItemToPickup))
        (CallFunction|SERVERDestroyActor (Variables|Default|GetItemToPickup))
        (if (> (Utilities|Array|Length _overlappingitems) 0)
          (Variables|Default|SetItemToPickup (.OutItem (Utilities|Array|Random _overlappingitems))))))
    (:then_1
      (return))))

(fn CreateItemAmountWidget
  (params (ItemToHandle :type BP%20Master%20Item%20Class%20Reference) (CurrentStack :type Integer))
  (bind _wb_itemamount (Variables|Default|GetWB%20ItemAmount)
    (:then
      (Widget|RemovefromParent _wb_itemamount))
    (:else
      (bind _returnvalue (UserInterface|CreateWidget "/Game/Components/Inventory/WB_ItemAmount.WB_ItemAmount_C" 0 (Variables|Default|GetInventory) ItemToHandle CurrentStack))
      (Variables|Default|SetWB%20ItemAmount _returnvalue)))
  (UserInterface|Viewport|AddtoViewport (Variables|Default|GetWB%20ItemAmount) 0)
  (bind _returnvalue_2 (Class|WidgetLayoutLibrary|GetMousePositiononViewport))
  (Class|UserWidget|SetPositioninViewport (Variables|Default|GetWB%20ItemAmount) (Math|Vector2D|MakeVector2D (.x _returnvalue_2) (.y _returnvalue_2)) false))