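; BP_MasterItem is a pickup item actor, apparently a base for inventory items.
; On InteractCollision overlap it passes itself to the other actor's AC_Inventory component, prints the item name and destroys itself.
; The construction script applies the physics setting and collision, and removes RotatingMovement unless enabled.
; BPI_Inventory interface check and message nodes exist but never run, so the component lookup is unguarded.
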(event OnComponentBeginOverlap(InteractCollision)
  (params (OverlappedComponent :type Primitive%20Component%20Object%20Reference) (OtherActor :type Actor%20Object%20Reference) (OtherComp :type Primitive%20Component%20Object%20Reference) (OtherBodyIndex :type Integer) (bFromSweep :type Boolean) (SweepResult :type Hit%20Result%20Structure%20%28by%20ref%29))
  (Default|AddItemtoInventory (Actor|GetComponentbyClass OtherActor "/Game/Components/Inventory/AC_Inventory.AC_Inventory_C") self)
  (Development|PrintString (Utilities|String|Append (Utilities|String|ToString(Text) (Variables|Default|GetItemName)) " added to inventory."))
  (Actor|DestroyActor))

(event EventBeginPlay)

(event Collision|EventActorBeginOverlap
  (params (OtherActor :type Actor%20Object%20Reference)))

(event EventTick
  (params (DeltaSeconds :type Float%20%28single-precision%29)))

(fn ConstructionScript
  (bind _staticmesh (Variables|Default|GetStaticMesh))
  (Utilities|FlowControl|Sequence
    (:then_0
      (Physics|SetSimulatePhysics _staticmesh (Variables|Default|GetSimulatePhysics?))
      (Collision|SetCollisionEnabled _staticmesh "QueryAndPhysics"))
    (:then_1
      (if (not (Variables|Default|GetUseRotatingComponent?))
        (Components|DestroyComponent (Variables|Default|GetRotatingMovement))))))